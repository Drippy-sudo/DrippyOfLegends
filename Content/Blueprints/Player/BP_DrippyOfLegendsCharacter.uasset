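; Player character for Drippy of Legends that moves to a given location and repeats a basic dagger attack on a target.
; An attack stops and disables movement, shows the dagger and starts a timer of the stab's length.
; The timer or a cancel restores walking, hides the dagger and attacks again if the target overlaps the range component.
; Construction attaches the dagger child actor to the right-hand socket, hidden.
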(event `self.MoveToLocation`
  (params (Location :type "Vector Structure"))
  ;[1 1 1] MoveTo
  (`AIBlueprintHelperLibrary.SimpleMoveToLocation` (`GameplayStatics.GetPlayerController` 0) Location))

(event `RepeatAttack`
  (bind _charactermovement (`self.CharacterMovement`))
  ;[1 1 1] Attack
  (if (not (`self.bIsAttacking`)) :!label _label
    (`CharacterMovementComponent.DisableMovement` _charactermovement)
    (`NavMovementComponent.StopActiveMovement` _charactermovement)
    (set `self.bIsAttacking` true)
    (`self.ToggleWeaponVisibility` true)
    (bind _returnvalue (`KismetSystemLibrary.K2_SetTimerDelegate` (delegate `ResetAttack`) (`self.Stab2Length`)))
    (set `self.AttackTimerHandle` _returnvalue)))

(event `self.PlayBasicAttack`
  ;[1 1 1] Attack
  (goto _label))

(event `ResetAttack`
  ;[1 1 1] Reset From Attack
  (set `self.bIsAttacking` false :!label _label_2)
  (`self.ToggleWeaponVisibility` false)
  (`CharacterMovementComponent.SetMovementMode` (`self.CharacterMovement`) "MOVE_Walking" 0)
  ;[1 1 1] Check to repeat attack
  (if (`PrimitiveComponent.IsOverlappingActor` (`self.BasicAttackRangeComp`) (`self.Target`))
    (`self.RepeatAttack`)))

(event `ToggleWeaponVisibility`
  (params (Toggle :type Boolean))
  ;[1 1 1] Toggle Weapon Visibility
  (`SceneComponent.SetVisibility` (`/Game/Blueprints/BP_Weapon.Weapon` (`self.DaggerRef`)) Toggle false))

(event `self.CancelAttack`
  ;[1 1 1] Cancel Attack
  (`KismetSystemLibrary.K2_ClearAndInvalidateTimerHandle` (`self.AttackTimerHandle`))
  (goto _label_2))

(fn `UserConstructionScript`
  (bind _returnvalue (`SceneComponent.K2_AttachToComponent` (`self.Weapon`) (`self.Mesh`) "RightHandIndex1" "KeepRelative" "KeepRelative" "KeepRelative" true))
  (if _returnvalue
    (bind _asbp_dagger (cast `/Game/Blueprints/BP_Dagger` (`ChildActorComponent.ChildActor` (`self.Weapon`))))
    (set `self.DaggerRef` _asbp_dagger)
    (`self.ToggleWeaponVisibility` false)))